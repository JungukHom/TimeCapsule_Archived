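; VR player character for motion-controller play, with thumbstick movement relative to the headset, object grabbing and a clue/inventory display.
; On BeginPlay it snaps to the ground by line trace, hides the clue widget and attaches a spawned Inventory.
; Left trigger toggles the clue, which blocks movement.
; Right trigger shows that widget when the right hand overlaps the inventory zone, otherwise grabs the nearest interface-implementing object until released, with haptic feedback.
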(event OnComponentBeginOverlap(InventoryCollision)
  (params (OverlappedComponent :type Primitive%20Component%20Object%20Reference) (OtherActor :type Actor%20Object%20Reference) (OtherComp :type Primitive%20Component%20Object%20Reference) (OtherBodyIndex :type Integer) (bFromSweep :type Boolean) (SweepResult :type Hit%20Result%20Structure%20%28by%20ref%29))
  ;[1 1 1] [InventoryCollision BeginEnd Overlap] Wants to See Inventory?
  (if (Utilities|Enum|Equal(Enum) (Utilities|GetDisplayName OtherComp) (Utilities|GetDisplayName (Variables|Default|GetCollision_RightHand)))
    (Variables|Default|SetWantsToSeeInventory true)
    (CallFunction|RumbleRightController 0.5)
    (bind _asgrabable_object (Utilities|Casting|CastToGrabableObject OtherActor))
    (if (not (Variables|/Game/TimeCapsule/Blueprints/GrabableObject.GrabableObject_C|GetIsGrabbed _asgrabable_object))
      (Default|AddItem (Variables|Default|GetInventory)))))

(event OnComponentEndOverlap(InventoryCollision)
  (params (OverlappedComponent :type Primitive%20Component%20Object%20Reference) (OtherActor :type Actor%20Object%20Reference) (OtherComp :type Primitive%20Component%20Object%20Reference) (OtherBodyIndex :type Integer))
  ;[1 1 1] [InventoryCollision BeginEnd Overlap] Wants to See Inventory?
  (if (Utilities|Enum|Equal(Enum) (Utilities|GetDisplayName OtherComp) (Utilities|GetDisplayName (Variables|Default|GetCollision_RightHand)))
    (Variables|Default|SetWantsToSeeInventory false)
    (CallFunction|RumbleRightController 0.5)))

(event Custom|RumbleLeftController
  (params (Scale :type Float%20%28single-precision%29))
  ;[1 1 1] [CustomEvent] Rumble Controller
  (Class|PlayerController|PlayHapticEffect (Game|GetPlayerController 0) "/Game/VirtualRealityBP/Blueprints/MotionControllerHaptics.MotionControllerHaptics" "Left" Scale false))

(event Custom|RumbleRightController
  (params (scale :type Float%20%28single-precision%29))
  ;[1 1 1] [CustomEvent] Rumble Controller
  (Class|PlayerController|PlayHapticEffect (Game|GetPlayerController 0) "/Game/VirtualRealityBP/Blueprints/MotionControllerHaptics.MotionControllerHaptics" "Right" scale false))

(event EventBeginPlay
  (bind _returnvalue (Transformation|GetActorLocation))
  (Utilities|FlowControl|Sequence
    (:then_0
      ;[1 1 1] [Initialize] Adjust Player's Z value
      (bind (_outhit _returnvalue_2) (Collision|LineTraceForObjects _returnvalue (+ _returnvalue "0.000000,0.000000,-1000.000000") (Utilities|Array|MakeArray "ObjectTypeQuery1" "ObjectTypeQuery2") false 0 "None"))
      (if _returnvalue_2
        (Transformation|SetActorLocation (.ImpactPoint (Collision|BreakHitResult _outhit)) false true)))
    (:then_1
      ;[1 1 1] [Initialize] Set Clue Visibillity
      (Rendering|SetVisibility (Variables|Default|GetClueWidget) false false)
      (Variables|Default|SetIsClueVisible false))
    (:then_2
      ;[1 1 1] [Initialize] Spawn and Attach Inventory Object
      (bind _returnvalue_3 (Game|SpawnActorfromClass "/Game/TimeCapsule/Blueprints/Inventory.Inventory_C" (Math|Transform|MakeTransform "0, 0,120.000000") "AlwaysSpawn" 0 0))
      (bind _output_get (Variables|Default|SetInventory _returnvalue_3))
      (Transformation|AttachComponentToComponent _output_get (Variables|Collision|GetCapsuleComponent) "None" "KeepRelative" "KeepRelative" "KeepRelative" true))))

(event Input|KeyboardEvents|MotionControllerRightThumbstickX
  (params (AxisValue :type Float%20%28single-precision%29))
  ;[1 1 1] Player Movement
  (if (Math|Boolean|Equal(Boolean) (Variables|Default|GetIsClueVisible) false)
    (Pawn|Input|AddMovementInput (Math|Vector|GetRightVector (Variables|Default|GetHMD)) (* AxisValue 0.25) true)))

(event Input|KeyboardEvents|MotionControllerRightThumbstickY
  (params (AxisValue :type Float%20%28single-precision%29))
  ;[1 1 1] Player Movement
  (if (Math|Boolean|Equal(Boolean) (Variables|Default|GetIsClueVisible) false)
    (Pawn|Input|AddMovementInput (Math|Vector|GetForwardVector (Variables|Default|GetHMD)) (* AxisValue -0.25) true)))

(event Input|KeyboardEvents|MotionControllerRightTrigger
  (params (Key :type Key%20Structure))
  (bind _cluewidget (Variables|Default|GetClueWidget))
  ;[1 1 1] [MotionController R Trigger] Show Inventory
  (:Pressed
    (if (Variables|Default|GetWantsToSeeInventory)
      (Rendering|SetVisibility _cluewidget true false)
      (else
        (CallFunction|Grab)
        (Variables|Default|SetIsGrabbed true)
        (for _index (range 0 100)
          (Development|PrintString (Utilities|GetDisplayName (Variables|Default|GetGrabbedObject)))))))
  (:Released
    (if (Variables|Default|GetWantsToSeeInventory)
      (Rendering|SetVisibility _cluewidget false false)
      (else
        (CallFunction|Release)
        (Variables|Default|SetIsGrabbed false)))))

(event Input|KeyboardEvents|MotionControllerLeftTrigger
  (params (Key :type Key%20Structure))
  ;[1 1 1] [MotionControoler L Trigger] Toggle Clue Visibillity
  (:Pressed
    (bind _output_get (Variables|Default|SetIsClueVisible (not (Variables|Default|GetIsClueVisible))))
    (CallFunction|SetClueVisibility _output_get)))

(event Input|KeyboardEvents|G
  (params (Key :type Key%20Structure))
  ;[1 1 1] [Event Dispatch] Widget
  (:Pressed
    (Default|CallGetItem)))

(fn ConstructionScript)

(fn GetViewingAngle
  (return (Transformation|GetWorldRotation (Variables|Default|GetHMD))))

(fn GetNearestActor
  (for _array_element (Collision|GetOverlappingActors (Variables|Default|GetCollision_RightHand) "/Script/Engine.Actor" :!class /Script/Engine.PrimitiveComponent)
    (if (Utilities|DoesObjectImplementInterface _array_element "/Game/TimeCapsule/Blueprints/GrabableObjectInterface.GrabableObjectInterface_C")
      (bind _output_get (LocalVariables|SetCurrentActor _array_element))
      (LocalVariables|SetCurrentLength (Math|Vector|VectorLength (- (Transformation|GetActorLocation _output_get) (Transformation|GetActorLocation))))
      (if (>= (LocalVariables|GetLength) (LocalVariables|GetCurrentLength))
        (LocalVariables|SetLength (LocalVariables|GetCurrentLength))
        (LocalVariables|SetNearestActor (LocalVariables|GetCurrentActor))
        (else
          (CallFunction|DoNothing)))))
  (return (LocalVariables|GetNearestActor)))

(fn Grab
  (if (not (Variables|Default|GetIsGrabbed))
    (bind _newparam (CallFunction|GetNearestActor))
    (Utilities|IsValid _newparam
      (:Is%20Valid
        (Variables|Default|SetGrabbedObject _newparam)
        (Class|PickupActorInterface|Pickup(Message) _newparam (Variables|Default|GetMotionController_Right))
        (CallFunction|RumbleRightController 0.0)
        (Variables|Default|SetIsGrabbed true)))))

(fn Release
  (if (Variables|Default|GetIsGrabbed)
    (Transformation|DetachFromComponent (Variables|/Script/Engine.Actor|GetRootComponent (Variables|Default|GetGrabbedObject)) "KeepRelative" "KeepRelative" "KeepWorld" true)
    (Variables|Default|SetIsGrabbed false)))

(fn Moveto
  (params (WorldPosition :type Vector))
  ;[1 1 1] TODO : Implement Fade In / Out
  (bind _returnvalue (Transformation|SetActorLocation WorldPosition false false))
  (return _returnvalue))

(fn SetClueVisibility
  (params (Visibillity :type Boolean))
  (Rendering|SetVisibility (Variables|Default|GetClueWidget) Visibillity false))

(fn GetActorLookRotation
  (return (Transformation|GetActorRotation)))