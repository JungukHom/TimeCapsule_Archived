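; GrabableObject is a physics prop that can be picked up and dropped in the TimeCapsule game.
; The construction script applies its configurable Mesh, and BeginPlay turns on physics simulation.
; PickUp disables physics and attaches the root to a given component, keeping its world transform.
; Drop re-enables physics and detaches the actor in place.
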(event EventPickUp
  (params (AttachTo :type Scene%20Component%20Object%20Reference))
  ;[1 1 1] Grab
  (Physics|SetSimulatePhysics (Variables|Debug|GetStaticMeshComponent) false)
  (Transformation|AttachComponentToComponent (Variables|Transformation|GetRootComponent) AttachTo "None" "KeepWorld" "KeepWorld" "KeepWorld" false))

(event EventDrop
  ;[1 1 1] Release
  (Physics|SetSimulatePhysics (Variables|Debug|GetStaticMeshComponent) true)
  (Transformation|DetachFromActor "KeepWorld" "KeepWorld" "KeepWorld"))

(event EventBeginPlay
  ;[1 1 1] Initialize
  (Physics|SetSimulatePhysics (Variables|Debug|GetStaticMeshComponent) true))

(fn ConstructionScript
  (Components|StaticMesh|SetStaticMesh (Variables|Debug|GetStaticMeshComponent) (Variables|Default|GetMesh)))