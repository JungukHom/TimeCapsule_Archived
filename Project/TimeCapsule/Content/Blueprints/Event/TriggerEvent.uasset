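; TriggerEvent is a trigger volume that fires an event when the player enters it.
; Its Box overlap passes the other actor to CheckIsPlayer, which casts to Player, and calls OnTriggerStarted on success.
; OnTriggerStarted is empty here, serving as a hook for the triggered behavior.
; The construction script applies TriggerScale as the box's world scale.
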(event OnComponentBeginOverlap(Box)
  (params (OverlappedComponent :type Primitive%20Component%20Object%20Reference) (OtherActor :type Actor%20Object%20Reference) (OtherComp :type Primitive%20Component%20Object%20Reference) (OtherBodyIndex :type Integer) (bFromSweep :type Boolean) (SweepResult :type Hit%20Result%20Structure%20%28by%20ref%29))
  (bind _result (CallFunction|CheckIsPlayer OtherActor))
  (if _result
    (CallFunction|OnTriggerStarted)))

(event Custom|OnTriggerStarted)

(fn ConstructionScript
  (Transformation|SetWorldScale3D (Variables|Default|GetBox) (Variables|Default|GetTriggerScale)))

(fn CheckIsPlayer
  (params (TriggeredActor :type Actor%20Object%20Reference))
  (Utilities|Casting|CastToPlayer TriggeredActor
    (:then
      (return true))
    (:CastFailed
      (return false))))