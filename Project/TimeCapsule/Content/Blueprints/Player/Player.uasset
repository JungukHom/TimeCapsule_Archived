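; VR player pawn that spawns motion controllers and a flashlight, and handles hand grabbing and thumbstick movement.
; BeginPlay drops the pawn to the ground with a downward trace, attaches left and right BP_MotionController actors to VROrigin, and spawns the flashlight at the left controller's flashlight position.
; Each trigger calls Grab or Release on its controller through GrabOrReleaseActor.
; The right thumbstick drives scaled-down movement along the HMD's forward and right vectors.
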(event EventBeginPlay
  (bind _returnvalue (Transformation|GetActorLocation))
  (Utilities|FlowControl|Sequence
    (:then_0
      ;[1 1 1] 높이 맞추기
      (bind (_outhit _returnvalue_2) (Collision|LineTraceForObjects _returnvalue (+ _returnvalue "0.000000,0.000000,-10000.000000") (Utilities|Array|MakeArray "ObjectTypeQuery1" "ObjectTypeQuery2") false 0 "None"))
      (if _returnvalue_2
        (Transformation|SetActorLocation (.ImpactPoint (Collision|BreakHitResult _outhit)) false true)))
    (:then_1
      ;[1 1 1] 모션컨트롤러 스폰 및 손전등 부착
      (Utilities|FlowControl|Sequence
        (:then_0
          (bind _returnvalue_3 (Game|SpawnActorfromClass "/Game/Blueprints/Player/BP_MotionController.BP_MotionController_C" (Math|Transform|MakeTransform "0, 0, 0") "AlwaysSpawn" self 0))
          (bind _output_get (Variables|Default|SetLeftController _returnvalue_3))
          (Transformation|AttachComponentToComponent _output_get (Variables|Default|GetVROrigin) "None" "SnapToTarget" "SnapToTarget" "KeepRelative" false)
          (Default|SetMotionSource _output_get "Left"))
        (:then_1
          (bind _returnvalue_4 (Game|SpawnActorfromClass "/Game/Blueprints/Player/BP_MotionController.BP_MotionController_C" (Math|Transform|MakeTransform "0,0.000000, 0") "AlwaysSpawn" self 0))
          (bind _output_get_2 (Variables|Default|SetRightController _returnvalue_4))
          (Transformation|AttachComponentToComponent _output_get_2 (Variables|Default|GetVROrigin) "None" "SnapToTarget" "SnapToTarget" "KeepRelative" false)
          (Default|SetMotionSource _output_get_2 "Right"))
        (:then_2
          (bind _position (Default|GetFlashLightPosition (Variables|Default|GetLeftController)))
          (bind _returnvalue_5 (Game|SpawnActorfromClass "/Game/Blueprints/Player/FlashLight.FlashLight_C" (Math|Transform|MakeTransform _position) "AlwaysSpawn" self 0))
          (bind _output_get_3 (Variables|Default|SetFlashLight _returnvalue_5))
          (Transformation|AttachComponentToComponent _output_get_3 0 "None" "SnapToTarget" "SnapToTarget" "KeepRelative" false))))))

(event Input|KeyboardEvents|MotionControllerRightThumbstickX
  (params (AxisValue :type Float%20%28single-precision%29))
  ;[1 1 1] 이동
  (Pawn|Input|AddMovementInput (Math|Vector|GetRightVector (Variables|Default|GetHMD)) (* AxisValue 0.25) true))

(event Input|KeyboardEvents|MotionControllerRightThumbstickY
  (params (AxisValue :type Float%20%28single-precision%29))
  ;[1 1 1] 이동
  (Pawn|Input|AddMovementInput (Math|Vector|GetForwardVector (Variables|Default|GetHMD)) (* (* AxisValue -1.0) 0.25) true))

(event Input|KeyboardEvents|MotionControllerLeftTrigger
  (params (Key :type Key%20Structure))
  ;[1 1 1] Get Input
  (:Pressed
    (Variables|Default|SetIsLeftHandTriggered true)
    (CallFunction|GraborReleaseActor (Variables|Default|GetLeftController) (Variables|Default|GetIsLeftHandTriggered) :!label _label))
  (:Released
    (Variables|Default|SetIsLeftHandTriggered false)
    (goto _label)))

(event Input|KeyboardEvents|MotionControllerRightTrigger
  (params (Key :type Key%20Structure))
  ;[1 1 1] Get Input
  (:Pressed
    (Variables|Default|SetIsRightHandTriggered true)
    (CallFunction|GraborReleaseActor (Variables|Default|GetRightController) (Variables|Default|GetIsRightHandTriggered) :!label _label))
  (:Released
    (Variables|Default|SetIsRightHandTriggered false)
    (goto _label)))

(fn ConstructionScript)

(fn GraborReleaseActor
  (params (MotionController :type BP%20Motion%20Controller%20Object%20Reference) (State :type Boolean))
  (if State
    (Default|Grab MotionController)
    (else
      (Default|Release MotionController))))