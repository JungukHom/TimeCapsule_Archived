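; VR player pawn for TimeCapsule that handles movement, interaction, clue inventory, collected keys and an adjustable spotlight.
; Pressing and tilting the left thumbstick moves relative to the HMD; grips and triggers message a nearby IInteractable from hand overlaps.
; Clues attach hidden under InventoryPosition for browsing and a murderer-diary count check.
; MoveTo teleports with camera fades and reveals the handlight and map, while widgets toggle by world scale.
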(event Custom|RumbleLeftController
  (params (Scale :type Float%20%28single-precision%29))
  ;[1 1 1] [CustomEvent] Rumble Controller
  (Class|PlayerController|PlayHapticEffect (Game|GetPlayerController 0) "/Game/VirtualRealityBP/Blueprints/MotionControllerHaptics.MotionControllerHaptics" "Left" Scale false))

(event Custom|RumbleRightController
  (params (scale :type Float%20%28single-precision%29))
  ;[1 1 1] [CustomEvent] Rumble Controller
  (Class|PlayerController|PlayHapticEffect (Game|GetPlayerController 0) "/Game/VirtualRealityBP/Blueprints/MotionControllerHaptics.MotionControllerHaptics" "Right" scale false))

(event EventBeginPlay
  (bind _returnvalue (Transformation|GetActorLocation))
  (Utilities|FlowControl|Sequence
    (:then_0
      ;[1 1 1] [Initialize] Adjust Player's Z value
      (bind (_outhit _returnvalue_2) (Collision|LineTraceForObjects _returnvalue (+ _returnvalue "0.000000,0.000000,-1000.000000") (Utilities|Array|MakeArray "ObjectTypeQuery1" "ObjectTypeQuery2") false 0 "None"))
      (if _returnvalue_2
        (Transformation|SetActorLocation (.ImpactPoint (Collision|BreakHitResult _outhit)) false true)))
    (:then_1
      (Class|HeadMountedDisplayFunctionLibrary|SetTrackingOrigin "Floor"))
    (:then_2
      (Widget|DisableAllOtherWidget))
    (:then_3
      (Rendering|SetVisibility (Variables|Default|Gethandlight) false true)
      (Rendering|SetVisibility (Variables|Default|Getmap) false true)
      (Rendering|SetVisibility (Variables|Default|GetSpotLight) false true)
      (Rendering|SetVisibility (Variables|Default|GetPointLight) false true))))

(event Input|KeyboardEvents|MotionControllerLeftThumbstickX
  (params (AxisValue :type Float%20%28single-precision%29))
  ;[1 1 1] Player Movement
  (if (Variables|Default|GetIsThumbstickPressed)
    (Pawn|Input|AddMovementInput (Math|Vector|GetRightVector (Variables|Default|GetHMD)) (* AxisValue 0.25) true)))

(event Input|KeyboardEvents|MotionControllerLeftThumbstickY
  (params (AxisValue :type Float%20%28single-precision%29))
  ;[1 1 1] Player Movement
  (if (Variables|Default|GetIsThumbstickPressed)
    (Pawn|Input|AddMovementInput (Math|Vector|GetForwardVector (Variables|Default|GetHMD)) (* AxisValue -0.25) true)))

(event Input|KeyboardEvents|MotionControllerRightTrigger
  (params (Key :type Key%20Structure))
  ;[1 1 1] Trigger Event
  (:Pressed
    (bind _nearestactor_ (Grab&Release|GetNearestActor (Variables|Default|GetCollision_RightHand)))
    (Utilities|IsValid _nearestactor_
      (:Is%20Valid
        (Class|IInteractable|OnTriggerPressed(Message) _nearestactor_ (Variables|Default|GetMotionController_Right))
        (Variables|Default|SetRightGrabbedObject _nearestactor_)
        (Variables|Default|SetIsRightGrabbed true))))
  (:Released
    (Utilities|IsValid (Variables|Default|GetRightGrabbedObject)
      (:Is%20Valid
        (Class|IInteractable|OnTriggerReleased(Message) (Variables|Default|GetRightGrabbedObject) (Variables|Default|GetMotionController_Right))))))

(event Input|KeyboardEvents|MotionControllerRightShoulder
  (params (Key :type Key%20Structure))
  (bind _inventoryposition (Variables|Default|GetInventoryPosition))
  (bind _returnvalue (Class|SceneComponent|GetNumChildrenComponents _inventoryposition))
  (:Pressed
    (CallFunction|Debug (Utilities|String|ToString(Integer) _returnvalue) 10 5.0)
    (if (>= _returnvalue 1)
      (bind _output_get (Variables|Default|SetIsClueVisible (not (Variables|Default|GetIsClueVisible))))
      (if _output_get
        (Clue|ShowClueatPosition (Variables|Default|GetClueIndex))
        (else
          (Clue|HideAllClues)
          (Variables|Default|SetClueIndex 0))))))

(event Input|KeyboardEvents|MotionControllerRightFaceButton2
  (params (Key :type Key%20Structure))
  (:Pressed
    (if (Variables|Default|GetIsClueVisible)
      (if (<= (Variables|Default|GetClueIndex) (- (Class|SceneComponent|GetNumChildrenComponents (Variables|Default|GetInventoryPosition)) 2))
        (bind _output_get (Variables|Default|SetClueIndex (+ (Variables|Default|GetClueIndex) 1))))
      (Clue|ShowClueatPosition _output_get))))

(event Input|KeyboardEvents|MotionControllerRightFaceButton4
  (params (Key :type Key%20Structure))
  (:Pressed
    (if (Variables|Default|GetIsClueVisible)
      (if (>= (Variables|Default|GetClueIndex) 1)
        (bind _output_get (Variables|Default|SetClueIndex (- (Variables|Default|GetClueIndex) 1))))
      (Clue|ShowClueatPosition _output_get))))

(event Input|KeyboardEvents|MotionControllerLeftThumbstick
  (params (Key :type Key%20Structure))
  ;[1 1 1] [Input] Thumbstick Pressed / Released
  (:Pressed
    (Variables|Default|SetIsThumbstickPressed true))
  (:Released
    (Variables|Default|SetIsThumbstickPressed false)))

(event Input|KeyboardEvents|MotionControllerRightGrip2
  (params (Key :type Key%20Structure))
  ;[1 1 1] Grip Item
  (:Pressed
    (bind _nearestactor_ (Grab&Release|GetNearestActor (Variables|Default|GetCollision_RightHand)))
    (Utilities|IsValid _nearestactor_
      (:Is%20Valid
        (Class|IInteractable|OnGripPressed(Message) _nearestactor_ (Variables|Default|GetMotionController_Right))))))

(event Input|KeyboardEvents|MotionControllerRightGrip1
  (params (Key :type Key%20Structure))
  ;[1 1 1] Grip Item
  (:Pressed
    (bind _nearestactor_ (Grab&Release|GetNearestActor (Variables|Default|GetCollision_RightHand)))
    (Utilities|IsValid _nearestactor_
      (:Is%20Valid
        (Class|IInteractable|OnGripPressed(Message) _nearestactor_ (Variables|Default|GetMotionController_Right))))))

(event Input|KeyboardEvents|MotionControllerLeftShoulder
  (params (Key :type Key%20Structure))
  (:Pressed
    (bind _output_get (Variables|Default|SetCurrentLightLevel (+ (Variables|Default|GetCurrentLightLevel) 1)))
    (switch int (Math|Integer|%(Integer) _output_get 5)
      (:0
        (bind _output_get_2 (Variables|Default|SetCurrentLightIntensity 5e+02))
        (Rendering|Components|Light|SetIntensity (Variables|Default|GetSpotLight) _output_get_2))
      (:1
        (bind _output_get_3 (Variables|Default|SetCurrentLightIntensity 1e+03))
        (Rendering|Components|Light|SetIntensity (Variables|Default|GetSpotLight) _output_get_3))
      (:2
        (bind _output_get_4 (Variables|Default|SetCurrentLightIntensity 1.5e+03))
        (Rendering|Components|Light|SetIntensity (Variables|Default|GetSpotLight) _output_get_4))
      (:3
        (bind _output_get_5 (Variables|Default|SetCurrentLightIntensity 2e+03))
        (Rendering|Components|Light|SetIntensity (Variables|Default|GetSpotLight) _output_get_5))
      (:4
        (bind _output_get_6 (Variables|Default|SetCurrentLightIntensity 2.5e+03))
        (Rendering|Components|Light|SetIntensity (Variables|Default|GetSpotLight) _output_get_6)))))

(event Input|KeyboardEvents|MotionControllerLeftTrigger
  (params (Key :type Key%20Structure))
  (bind _motioncontroller_left (Variables|Default|GetMotionController_Left))
  ;[1 1 1] Trigger Event
  (:Pressed
    (bind _nearestactor_ (Grab&Release|GetNearestActor (Variables|Default|GetCollision_LeftHand)))
    (Utilities|IsValid _nearestactor_
      (:Is%20Valid
        (Class|IInteractable|OnTriggerPressed(Message) _nearestactor_ _motioncontroller_left)
        (Variables|Default|SetLeftGrabbedObject _nearestactor_)
        (Variables|Default|SetIsLeftGrabbed true))))
  (:Released
    (Utilities|IsValid (Variables|Default|GetLeftGrabbedObject)
      (:Is%20Valid
        (Class|IInteractable|OnTriggerReleased(Message) (Variables|Default|GetLeftGrabbedObject) _motioncontroller_left)
        (Variables|Default|SetIsLeftGrabbed false)))))

(fn ConstructionScript)

(fn GetActorLookRotation
  (return (Transformation|GetWorldRotation (Variables|Default|GetHMD))))

(fn GetNearestActor
  (params (Collision :type Sphere%20Component%20Object%20Reference))
  (for _array_element (Collision|GetOverlappingActors Collision "/Script/Engine.Actor" :!class /Script/Engine.PrimitiveComponent)
    (if (Utilities|DoesObjectImplementInterface _array_element "/Game/TimeCapsule/NewBlurprints/IInteractable.IInteractable_C")
      (bind _output_get (LocalVariables|SetCurrentActor _array_element))
      (LocalVariables|SetCurrentLength (Math|Vector|VectorLength (- (Transformation|GetActorLocation _output_get) (+ (Transformation|GetActorLocation) (Variables|/Script/Engine.SceneComponent|GetRelativeLocation (Variables|Default|GetMotionController_Right))))))
      (if (>= (LocalVariables|GetLength) (LocalVariables|GetCurrentLength))
        (LocalVariables|SetLength (LocalVariables|GetCurrentLength))
        (LocalVariables|SetNearestActor (LocalVariables|GetCurrentActor))
        (else
          (CallFunction|DoNothing)))))
  (return (LocalVariables|GetNearestActor)))

(fn Grab
  (params (Controller :type Motion%20Controller%20Component%20Object%20Reference) (Collision :type Sphere%20Component%20Object%20Reference))
  (bind _nearestactor_ (Grab&Release|GetNearestActor Collision))
  (Utilities|IsValid _nearestactor_
    (:Is%20Valid
      (bind _output_get (Variables|Default|SetLeftGrabbedObject _nearestactor_))
      (Class|IGrabbable|PickUp(Message) _output_get Controller)
      (CallFunction|RumbleRightController 0.5)
      (Variables|Default|SetIsRightGrabbed true))))

(fn Release
  (if (Variables|Default|GetIsRightGrabbed)
    (Class|IGrabbable|Drop(Message) (Variables|Default|GetLeftGrabbedObject))
    (Variables|Default|SetIsRightGrabbed false)))

(fn Moveto
  (params (WorldPosition :type Vector))
  (CameraFades|StartCameraFade :self (Game|GetPlayerCameraManager 0) :ToAlpha 1.0 :Duration 2.0 :bShouldFadeAudio true)
  (bind _returnvalue (Transformation|SetActorLocation WorldPosition false true))
  (Rendering|SetVisibility (Variables|Default|Gethandlight) true true)
  (Rendering|SetVisibility (Variables|Default|Getmap) true true)
  (Rendering|SetVisibility (Variables|Default|GetSpotLight) true true)
  (Rendering|SetVisibility (Variables|Default|GetPointLight) true true)
  (CameraFades|StartCameraFade :self (Game|GetPlayerCameraManager 0) :FromAlpha 1.0 :Duration 2.0 :bShouldFadeAudio true)
  (return _returnvalue))

(fn GetGrabbingController
  (Utilities|FlowControl|Sequence
    (:then_0
      (if (Variables|Default|GetIsLeftGrabbed)
        (return (Variables|Default|GetMotionController_Left))))
    (:then_1
      (if (Variables|Default|GetIsRightGrabbed)
        (return (Variables|Default|GetMotionController_Right))))))

(fn AddClue
  (params (Item :type Clue%20Object%20Reference))
  (bind _output_get (LocalVariables|Set_Item Item))
  (bind _output (Default|GetStaticMesh _output_get))
  (bind _returnvalue (Transformation|AttachComponentToComponent _output (Variables|Default|GetInventoryPosition) "None" "KeepRelative" "KeepRelative" "KeepRelative" true))
  (if _returnvalue
    (Physics|SetSimulatePhysics (Variables|/Game/TimeCapsule/NewBlurprints/GrabbableObject.GrabbableObject_C|GetStaticMesh (LocalVariables|Get_Item)) false)
    (Rendering|SetVisibility (Variables|/Game/TimeCapsule/NewBlurprints/GrabbableObject.GrabbableObject_C|GetStaticMesh (LocalVariables|Get_Item)) false true)
    (else
      (CallFunction|DoNothing))))

(fn AddKey
  (params (Key :type KeyEnum%20Enum :default "NewEnumerator0"))
  (Utilities|Array|AddUnique (Variables|Default|GetCollectedKeys) Key))

(fn ShowClueatPosition
  (params (Index :type Integer))
  (bind _inventoryposition (Variables|Default|GetInventoryPosition))
  (bind _inventoryposition_2 (Variables|Default|GetInventoryPosition))
  (bind _returnvalue (Class|SceneComponent|GetNumChildrenComponents _inventoryposition))
  (bind _returnvalue_2 (Math|Integer|%(Integer) Index _returnvalue))
  (bind _returnvalue_3 (Math|Integer|Absolute(Integer) _returnvalue_2))
  (bind _returnvalue_4 (Components|GetChildComponent _inventoryposition_2 _returnvalue_3))
  (Clue|HideAllClues)
  (if (Utilities|DoesObjectImplementInterface _returnvalue_4 "/Game/TimeCapsule/NewBlurprints/IInteractable.IInteractable_C")
    (Class|IInteractable|OtherFunction(Message) _returnvalue_4)))

(fn HideAllClues
  (for _array_element (Components|GetChildrenComponents (Variables|Default|GetInventoryPosition) false)
    (Rendering|SetVisibility _array_element false true)))

(fn ShowWidget
  (params (Index :type Integer))
  (if (and (>= Index 0) (<= Index (Class|SceneComponent|GetNumChildrenComponents (Variables|Default|GetWidgetPosition))))
    (Transformation|SetWorldScale3D (Components|GetChildComponent (Variables|Default|GetWidgetPosition) Index) "1.000000,1.000000,1.000000")))

(fn DisableAllOtherWidget
  (for _array_element (Components|GetChildrenComponents (Variables|Default|GetWidgetPosition) false)
    (Transformation|SetWorldScale3D _array_element "0, 0, 0")))

(fn HasKey
  (params (Key :type KeyEnum%20Enum :default "NewEnumerator0"))
  (for _array_element (Variables|Default|GetCollectedKeys)
    (if (Utilities|Enum|Equal(Enum) _array_element Key)
      (return true)))
  (return false))

(fn CheckMurdererDiaryCount
  (for _array_element (Components|GetChildrenComponents (Variables|Default|GetInventoryPosition) false)
    (if (Utilities|String|Contains (Utilities|GetDisplayName _array_element) "ClueDiary")
      (LocalVariables|SetCount (+ (LocalVariables|GetCount) 1))))
  (if (>= (LocalVariables|GetCount) 5)
    (return true)
    (else
      (return false))))