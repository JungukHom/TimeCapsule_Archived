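; BP_DestructibleObj is a physics-simulated destructible prop that can be picked up, dropped and smashed, with its mesh assigned in the construction script.
; PickUp turns off physics and attaches it to the given component; Drop detaches it and restores physics.
; Component hits derive impact strength from velocity, scaling hit-sound volume and, above a higher threshold, calling Destruct to play a sound and apply damage with a reversed-velocity impulse.
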(event OnComponentHit(Destructible)
  (params (HitComponent :type Primitive%20Component%20Object%20Reference) (OtherActor :type Actor%20Object%20Reference) (OtherComp :type Primitive%20Component%20Object%20Reference) (NormalImpulse :type Vector :default "0, 0, 0") (Hit :type Hit%20Result%20Structure%20%28by%20ref%29))
  (bind _destructible (Variables|Default|GetDestructible))
  (bind _returnvalue (Transformation|GetComponentVelocity _destructible))
  (bind _returnvalue_2 (Math|Vector|VectorLength _returnvalue))
  (bind _returnvalue_3 (/ _returnvalue_2 1e+02))
  ;[1 1 1] OnComponentHit => Hit || Destroy
  (Utilities|FlowControl|Sequence
    (:then_0
      ;;[1 1 1] Play Hitsound when (0.3 <= value <= 1)
      (if (>= _returnvalue_3 0.3)
        (CallFunction|PlayHitSound (Math|Float|Clamp(Float) _returnvalue_3))))
    (:then_1
      ;;[1 1 1] Destruct when (value >= 1)
      (if (>= _returnvalue_3 1.0)
        (CallFunction|Destruct _returnvalue_3 (* _returnvalue -1.0))))))

(event EventPlayHitSound
  (params (Volume :type Float%20%28single-precision%29))
  ;[1 1 1] Play Hit Sound
  (Audio|PlaySoundatLocation (Variables|Default|GetHitSound) (Transformation|GetActorLocation) "0, 0, 0" Volume 1.0 0.0 0 0 0))

(event EventDestruct
  (params (Force :type Float%20%28single-precision%29) (Velocity :type Vector :default "0, 0, 0"))
  (bind _returnvalue (* Force 1e+02))
  (bind _destructible (Variables|Default|GetDestructible))
  ;[1 1 1] Destruct
  (CallFunction|PlayDestructSound)
  (Class|DestructibleComponent|ApplyDamage _destructible _returnvalue (Transformation|GetWorldLocation _destructible) Velocity _returnvalue))

(event EventPlayDestructSound
  ;[1 1 1] Play Destruct Sound
  (Audio|PlaySoundatLocation (Variables|Default|GetDestroySound) (Transformation|GetActorLocation) "0, 0, 0" 1.0 1.0 0.0 0 0 0))

(event EventPickUp
  (params (AttachTo :type Scene%20Component%20Object%20Reference))
  ;[1 1 1] Grab
  (Physics|SetSimulatePhysics (Variables|Default|GetDestructible) false)
  (bind _returnvalue (Transformation|AttachComponentToComponent (Variables|Transformation|GetRootComponent) AttachTo "None" "KeepWorld" "KeepWorld" "KeepWorld" false))
  (if _returnvalue
    (Variables|Default|SetIsGrabbed true)))

(event EventDrop
  ;[1 1 1] Release
  (Physics|SetSimulatePhysics (Variables|Default|GetDestructible) true)
  (Transformation|DetachFromActor "KeepWorld" "KeepWorld" "KeepWorld")
  (Variables|Default|SetIsGrabbed false))

(event EventBeginPlay
  ;[1 1 1] BeginPlay : Set Simulate Physics & Enable Collision
  (Physics|SetSimulatePhysics (Variables|Default|GetDestructible) true)
  (Collision|SetCollisionEnabled (Variables|Default|GetDestructible) "QueryAndPhysics"))

(fn ConstructionScript
  (Class|DestructibleComponent|SetDestructibleMesh (Variables|Default|GetDestructible) (Variables|Default|GetMesh))
  (Physics|SetSimulatePhysics (Variables|Default|GetDestructible) true))