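; DoorTest is a test Blueprint for a grabbable door that swings with trigger input.
; Trigger press stores the controller and disables door physics; release clears it and restores physics.
; While held, Tick smoothly interpolates the door's yaw toward the player character's location, not the stored controller.
; Each tick also prints the yaw change since the previous frame, which is not applied to physics.
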(event Custom|OnTriggerPressed
  (params (PressedController :type Motion%20Controller%20Object%20Reference))
  (Variables|Default|SetOnControlled? true)
  (Variables|Default|SetOwnerController PressedController)
  (Physics|SetSimulatePhysics (Variables|Default|GetDoor) false))

(event Custom|OnTriggerReleased
  (Variables|Default|SetOnControlled? false)
  (Variables|Default|SetOwnerController 0)
  (Physics|SetSimulatePhysics (Variables|Default|GetDoor) true))

(event EventTick
  (params (DeltaSeconds :type Float%20%28single-precision%29))
  (Utilities|FlowControl|Sequence
    (:then_1
      (if (Variables|Default|GetOnControlled?)
        ;[1 1 1] 문이 컨트롤되고 있을때
        (Utilities|FlowControl|Sequence
          (:then_0
            ;;[1 1 1] 콘트롤러 위치로부터 문이 향해야 할 방향을 결정
            (Variables|Default|SetTargetRot (Math|Rotator|MakeRotator 0.0 0.0 (.yaw (Math|Rotator|FindLookatRotation (Transformation|GetWorldLocation (Variables|Default|GetDoor)) (Transformation|GetActorLocation (Game|GetPlayerCharacter 0)))))))
          (:then_1
            (Variables|Default|SetCurrentDoorRot (Math|Interpolation|RInterpTo (Variables|Default|GetCurrentDoorRot) (Variables|Default|GetTargetRot) (Utilities|Time|GetWorldDeltaSeconds) 2e+01)))
          (:then_2
            ;[1 1 1] 현재로테이션으로 문위치 회전
            (Transformation|SetWorldRotation (Variables|Default|GetDoor) (Variables|Default|GetCurrentDoorRot) false false)))))
    (:then_2
      (bind _output_get (Variables|Default|SetCurrentAngular (.yaw (Math|Rotator|Delta(Rotator) (Variables|Default|GetCurrentDoorRot) (Variables|Default|GetPreviousDoorRot)))))
      (Development|PrintString (Utilities|String|ToString(Float) _output_get)))
    (:then_4
      (Variables|Default|SetPreviousDoorRot (Variables|Default|GetCurrentDoorRot)))))

(fn ConstructionScript)