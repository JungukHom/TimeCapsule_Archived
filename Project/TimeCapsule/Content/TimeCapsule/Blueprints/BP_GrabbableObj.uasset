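; Base grabbable physics object that can be picked up by attaching it to a given component and dropped again.
; PickUp turns off physics, attaches keeping world transform, flags it as grabbed and plays a grab sound; Drop detaches and restores physics.
; Component hits pass a speed-scaled, thresholded volume to PlayHitSound, but that event's sound node is disconnected.
; The construction script's mesh assignment is also disconnected.
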(event OnComponentHit(StaticMeshComponent)
  (params (HitComponent :type Primitive%20Component%20Object%20Reference) (OtherActor :type Actor%20Object%20Reference) (OtherComp :type Primitive%20Component%20Object%20Reference) (NormalImpulse :type Vector :default "0, 0, 0") (Hit :type Hit%20Result%20Structure%20%28by%20ref%29))
  (bind _staticmeshcomponent (Variables|Debug|GetStaticMeshComponent))
  (bind _returnvalue (Transformation|GetComponentVelocity _staticmeshcomponent))
  (bind _returnvalue_2 (Math|Vector|VectorLength _returnvalue))
  (bind _returnvalue_3 (/ _returnvalue_2 5e+02))
  (bind _returnvalue_4 (Math|Float|Clamp(Float) _returnvalue_3))
  ;[1 1 1] OnComponentHit => Play Hit Sound
  (if (>= _returnvalue_4 0.5)
    (CallFunction|PlayHitSound _returnvalue_4)))

(event EventPlayHitSound
  (params (Volume :type Float%20%28single-precision%29))
  ;[1 1 1] Play Hit Sound
)

(event EventPickUp
  (params (AttachTo :type Scene%20Component%20Object%20Reference))
  ;[1 1 1] Grab
  (Physics|SetSimulatePhysics (Variables|Debug|GetStaticMeshComponent) false)
  (bind _returnvalue (Transformation|AttachComponentToComponent (Variables|Transformation|GetRootComponent) AttachTo "None" "KeepWorld" "KeepWorld" "KeepWorld" false))
  (if _returnvalue
    (Variables|Default|SetIsGrabbed true)
    (Audio|PlaySoundatLocation (Variables|Default|GetGrabSound) (Transformation|GetActorLocation) "0, 0, 0" (Variables|Default|GetGrabSoundMultiplier) 1.0 0.0 0 0 0)))

(event EventDrop
  ;[1 1 1] Release
  (Physics|SetSimulatePhysics (Variables|Debug|GetStaticMeshComponent) true)
  (Transformation|DetachFromActor "KeepRelative" "KeepRelative" "KeepWorld")
  (Variables|Default|SetIsGrabbed false))

(event EventBeginPlay
  ;[1 1 1] Initialize
  (Physics|SetSimulatePhysics (Variables|Debug|GetStaticMeshComponent) true)
  (Variables|/Script/Engine.PrimitiveComponent|SetbGenerateOverlapEvents (Variables|Debug|GetStaticMeshComponent) true))

(fn ConstructionScript)

(fn GetStaticMesh
  (return (Variables|Default|GetMesh)))