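; Door_Last is a key-locked door that opens for the VR player.
; When a BP_VRPlayer enters the Box trigger, it searches that player's MyKeys for an entry matching its Key.
; A match plays a timeline that drives the actor's roll, keeping its current pitch and yaw.
; The graph has no closing or reverse logic.
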(event OnComponentBeginOverlap(Box)
  (params (OverlappedComponent :type Primitive%20Component%20Object%20Reference) (OtherActor :type Actor%20Object%20Reference) (OtherComp :type Primitive%20Component%20Object%20Reference) (OtherBodyIndex :type Integer) (bFromSweep :type Boolean) (SweepResult :type Hit%20Result%20Structure%20%28by%20ref%29))
  (bind _returnvalue (Transformation|GetActorRotation))
  (bind (_roll _pitch _yaw) (Math|Rotator|BreakRotator _returnvalue))
  (bind _asbp_vrplayer (Utilities|Casting|CastToBP_VRPlayer OtherActor))
  (for _array_element (Variables|/Game/TimeCapsule/Blueprints/BP_VRPlayer.BP_VRPlayer_C|GetMyKeys _asbp_vrplayer)
    (if (Utilities|Enum|Equal(Enum) _array_element (Variables|Default|GetKey))
      (bind _newtrack_0 (Timeline|Timeline_0 Play)
        (:Update
          (Transformation|SetActorRotation (Math|Rotator|MakeRotator _newtrack_0 _pitch _yaw)))))))

(event EventBeginPlay)

(event Collision|EventActorBeginOverlap
  (params (OtherActor :type Actor%20Object%20Reference)))

(event EventTick
  (params (DeltaSeconds :type Float%20%28single-precision%29)))

(fn ConstructionScript)