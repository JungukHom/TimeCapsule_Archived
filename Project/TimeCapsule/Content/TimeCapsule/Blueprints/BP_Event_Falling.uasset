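; Event actor that makes a target static mesh fall when the player enters its trigger.
; On BeginPlay it turns off physics simulation on the target's mesh component so the object holds in place.
; An overlap on the Collision component passes a player check, then calls Fall, which turns physics simulation on.
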(event OnComponentBeginOverlap(Collision)
  (params (OverlappedComponent :type Primitive%20Component%20Object%20Reference) (OtherActor :type Actor%20Object%20Reference) (OtherComp :type Primitive%20Component%20Object%20Reference) (OtherBodyIndex :type Integer) (bFromSweep :type Boolean) (SweepResult :type Hit%20Result%20Structure%20%28by%20ref%29))
  (bind _result (CallFunction|CheckIsPlayer OtherActor))
  (if _result
    (CallFunction|Fall)
    (else
      (CallFunction|DoNothing))))

(event EventBeginPlay
  (Physics|SetSimulatePhysics (Variables|/Script/Engine.StaticMeshActor|GetStaticMeshComponent (Variables|Default|GetTarget)) false))

(fn ConstructionScript)

(fn Fall
  (Physics|SetSimulatePhysics (Variables|/Script/Engine.StaticMeshActor|GetStaticMeshComponent (Variables|Default|GetTarget)) true))