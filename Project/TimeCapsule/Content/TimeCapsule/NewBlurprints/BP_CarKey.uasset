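; BP_CarKey is a grabbable car key for VR that also triggers loading of the next streamed level.
; PickUp stops physics and attaches it to the given component; Drop restores physics and detaches it, both updating IsGrabbed.
; Tick ignores IsGrabbed: its condition is always true, so after two seconds it requests a blocking NextLevelName load every frame while the pawn is a VRPlayer.
; Move, VR-reset and destroy logic is disconnected.
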(event EventBeginPlay
  (|CallParentFunction) ; This node is disabled and will not be called.\nDrag off pins to build functionality.
)

(event EventTick
  (params (DeltaSeconds :type Float%20%28single-precision%29))
  (if true
    (Variables|Default|SetGrabbedTime (+ DeltaSeconds (Variables|Default|GetGrabbedTime)))
    (if (>= (Variables|Default|GetGrabbedTime) 2.0)
      (Utilities|Casting|CastToVRPlayer (Game|Player|GetPlayerPawn 0))
      (Game|LoadStreamLevel(byName) (Variables|Default|GetNextLevelName) true true))
    (else
      (CallFunction|DoNothing))))

(event EventPickUp
  (params (AttachTo :type Scene%20Component%20Object%20Reference))
  ;[1 1 1] Grab
  (Physics|SetSimulatePhysics (Variables|Default|GetStaticMeshComponent) false)
  (bind _returnvalue (Transformation|AttachComponentToComponent (Variables|Transformation|GetRootComponent) AttachTo "None" "KeepWorld" "KeepWorld" "KeepWorld" false))
  (if _returnvalue
    (Variables|Default|SetIsGrabbed true)))

(event EventDrop
  ;[1 1 1] Release
  (Physics|SetSimulatePhysics (Variables|Default|GetStaticMeshComponent) true)
  (Transformation|DetachFromActor "KeepRelative" "KeepRelative" "KeepWorld")
  (Variables|Default|SetIsGrabbed false))

(fn ConstructionScript
  (|CallParentFunction))